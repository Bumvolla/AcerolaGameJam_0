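; BP_Architecture is a level geometry actor that gets a decal mark wherever a BP_Aberration hits it.
; Its static mesh's hit event filters for that actor and spawns a BP_Cum decal actor at the impact point, oriented along the surface normal.
; The decal's height and width scale linearly with the Aberration capsule's speed, while its projection depth stays thin and fixed.
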(event `self.StaticMesh.OnComponentHit`
  (params (HitComponent :type "PrimitiveComponent Object Reference") (OtherActor :type "Actor Object Reference") (OtherComp :type "PrimitiveComponent Object Reference") (NormalImpulse :type "Vector Structure") (Hit :type "HitResult Structure (by ref)"))
  (bind (_bblockinghit _binitialoverlap _time _distance _location _impactpoint _normal _impactnormal) (`GameplayStatics.BreakHitResult` Hit))
  (bind _asbp_aberration (cast `/Game/AcerolaJam/BP/BP_Aberration` OtherActor))
  (bind _returnvalue (`|SpawnActorFromClass` "/Game/AcerolaJam/BP/BP_Cum.BP_Cum_C" (`KismetMathLibrary.MakeTransform` _impactpoint (`KismetMathLibrary.Conv_VectorToRotator` _impactnormal)) "Undefined" "OverrideRootScale" null null))
  (bind _returnvalue_2 (/ (`KismetMathLibrary.VSize` (`SceneComponent.GetComponentVelocity` (`Character.CapsuleComponent` _asbp_aberration))) 1500.0))
  (`SceneComponent.SetRelativeScale3D` (`/Game/AcerolaJam/BP/BP_Cum.Decal` _returnvalue) (`KismetMathLibrary.MakeVector` 0.01 _returnvalue_2 _returnvalue_2)))

(fn `UserConstructionScript`)