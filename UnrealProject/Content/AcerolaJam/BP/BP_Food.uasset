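; BP_Food is an AI prey character that flees or panics on sight of BP_Aberration and heals it when caught.
; Pawn sensing sets the "HasSeenPlayer?" blackboard key, flags the ABP_Enemy anim instance as scared and raises walk speed.
; A mesh hit by the Aberration heals it once, flags death on the anim instance, disables movement, then switches to a physics body after a delay.
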(event `self.Mesh.OnComponentHit`
  (params (HitComponent :type "PrimitiveComponent Object Reference") (OtherActor :type "Actor Object Reference") (OtherComp :type "PrimitiveComponent Object Reference") (NormalImpulse :type "Vector Structure") (Hit :type "HitResult Structure (by ref)"))
  (bind _mesh (`self.Mesh`))
  (if (not (`/Game/AcerolaJam/BP/ABP_Enemy.HasDied?` (`self.As ABP Enemy`)))
    (bind _asbp_aberration (cast `/Game/AcerolaJam/BP/BP_Aberration` OtherActor))
    (`/Game/AcerolaJam/BP/BP_Aberration.Heal` _asbp_aberration (`self.HealingAmmount`))
    (set `/Game/AcerolaJam/BP/ABP_Enemy.HasDied?` true (`self.As ABP Enemy`))
    (`CharacterMovementComponent.DisableMovement` (`self.CharacterMovement`))
    (`KismetSystemLibrary.Delay` 3.0)
    (`PrimitiveComponent.SetSimulatePhysics` _mesh true)
    (`PrimitiveComponent.SetCollisionObjectType` _mesh "ECC_PhysicsBody")))

(event `self.PawnSensing.OnSeePawn`
  (params (Pawn :type "Pawn Object Reference"))
  (cast `/Game/AcerolaJam/BP/BP_Aberration` Pawn)
  (`BlackboardComponent.SetValueAsBool` (`AIBlueprintHelperLibrary.GetBlackboard` (`AIBlueprintHelperLibrary.GetAIController` self)) "HasSeenPlayer?" true)
  (set `/Game/AcerolaJam/BP/ABP_Enemy.IsScared?` true (`self.As ABP Enemy`))
  (set `CharacterMovementComponent.MaxWalkSpeed` 600.0 (`self.CharacterMovement`)))

(event `self.ReceiveBeginPlay`
  (bind _asabp_enemy (cast `/Game/AcerolaJam/BP/ABP_Enemy` (`SkeletalMeshComponent.GetAnimInstance` (`self.Mesh`))))
  (set `self.As ABP Enemy` _asabp_enemy))

(fn `UserConstructionScript`)